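; StatsTrackerLibrary is a set of helper functions for tracking named stats on the game instance.
; GetStats casts the game instance to Instance_save, whose Stats map holds the values.
; AddStat adds the value to an existing entry or creates one if the name is missing.
; ReadStat returns the map's value for a name without checking that it exists.
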(fn `AddStat`
  (params (StatName :type String) (Value :type "Float (double-precision)"))
  (bind _gameinstance (`self.GetStats` null))
  (bind _stats (`/Game/Robert_Green_Bps/Instance_save.Stats` _gameinstance))
  (bind (_value _returnvalue) (`BlueprintMapLibrary.Map_Find` _stats StatName))
  (if _returnvalue
    (`BlueprintMapLibrary.Map_Add` _stats (`local.StatName`) (+ (`local.Value`) _value))
    (else
      (`BlueprintMapLibrary.Map_Add` _stats (`local.StatName`) (`local.Value`)))))

(fn `GetStats`
  (returns (GameInstance :type "/Game/Robert_Green_Bps/Instance_save Object Reference"))
  (bind _asinstance_save (cast `/Game/Robert_Green_Bps/Instance_save` (`GameplayStatics.GetGameInstance` null)))
  (return _asinstance_save))

(fn `ReadStat`
  (params (StatName :type String))
  (returns (Value :type "Float (double-precision)"))
  (bind _gameinstance (`self.GetStats` null))
  (return (`BlueprintMapLibrary.Map_Find` (`/Game/Robert_Green_Bps/Instance_save.Stats` _gameinstance) (`local.StatName`))))