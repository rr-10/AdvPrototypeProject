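; Wall light for a Red Light Green Light game, cycling its material between red and green with countdown, stop and go sounds.
; Tick feeds a three-second Delay into a FlipFlop, alternating between a yellow-red blink that ends on red and solid green.
; BeginPlay separately runs an endless Delay chain of 2D audio cues, matched to the light only by timing.
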(event `self.ReceiveTick`
  (params (DeltaSeconds :type "Float (single-precision)"))
  ;[1 1 1] RED LIGHT GREEN LIGHT
  (`KismetSystemLibrary.Delay` 3.0)
  (`/Engine/EditorBlueprintResources/StandardMacros.FlipFlop`
    (:`A`
      (`PrimitiveComponent.SetMaterial` (`self.wall_light`) 0 "/Game/Remo/Materials/MI_Yellow.MI_Yellow")
      (`KismetSystemLibrary.Delay` 0.2)
      (`PrimitiveComponent.SetMaterial` (`self.wall_light`) 0 "/Game/Remo/Materials/MI_Red.MI_Red")
      (`KismetSystemLibrary.Delay` 0.2)
      (`PrimitiveComponent.SetMaterial` (`self.wall_light`) 0 "/Game/Remo/Materials/MI_Yellow.MI_Yellow")
      (`KismetSystemLibrary.Delay` 0.2)
      (`PrimitiveComponent.SetMaterial` (`self.wall_light`) 0 "/Game/Remo/Materials/MI_Red.MI_Red")
      (`KismetSystemLibrary.Delay` 0.2)
      (`PrimitiveComponent.SetMaterial` (`self.wall_light`) 0 "/Game/Remo/Materials/MI_Yellow.MI_Yellow")
      (`KismetSystemLibrary.Delay` 0.2)
      (`PrimitiveComponent.SetMaterial` (`self.wall_light`) 0 "/Game/Remo/Materials/MI_Red.MI_Red"))
    (:`B`
      (`PrimitiveComponent.SetMaterial` (`self.wall_light`) 0 "/Game/Remo/Materials/MI_Green.MI_Green"))))

(event `self.ReceiveBeginPlay`
  (`KismetSystemLibrary.Delay` 1.0 :!label _label)
  (`GameplayStatics.PlaySound2D` "/Game/SarahRoddam_Audio/SFX_Puzzles/SFX_RedGreenLight_Countdown_Cue.SFX_RedGreenLight_Countdown_Cue" 1.0 1.0 0.0 null null)
  (`KismetSystemLibrary.Delay` 1.0)
  (`GameplayStatics.PlaySound2D` "/Game/SarahRoddam_Audio/SFX_Puzzles/SFX_RedGreenLight_Countdown_Cue.SFX_RedGreenLight_Countdown_Cue" 1.0 1.0 0.0 null null)
  (`KismetSystemLibrary.Delay` 1.0)
  (`GameplayStatics.PlaySound2D` "/Game/SarahRoddam_Audio/SFX_Puzzles/SFX_RedGreenLight_Countdown_Cue.SFX_RedGreenLight_Countdown_Cue" 1.0 1.0 0.0 null null)
  (`KismetSystemLibrary.Delay` 1.0)
  (`GameplayStatics.PlaySound2D` "/Game/SarahRoddam_Audio/SFX_Puzzles/SFX_RedGreenLight_Stop_Cue.SFX_RedGreenLight_Stop_Cue" 1.0 1.0 0.0 null null)
  (`KismetSystemLibrary.Delay` 1.0)
  (`GameplayStatics.PlaySound2D` "/Game/SarahRoddam_Audio/SFX_Puzzles/SFX_RedGreenLight_Countdown_Cue.SFX_RedGreenLight_Countdown_Cue" 1.0 1.0 0.0 null null)
  (`KismetSystemLibrary.Delay` 1.0)
  (`GameplayStatics.PlaySound2D` "/Game/SarahRoddam_Audio/SFX_Puzzles/SFX_RedGreenLight_Go_Cue.SFX_RedGreenLight_Go_Cue" 1.0 1.0 0.0 null null)
  (goto _label))

(fn `UserConstructionScript`)