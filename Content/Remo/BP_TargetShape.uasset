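; BP_TargetShape is a target shape actor whose mesh and colour are chosen through Shape and Colour variables.
; The construction script sets the static mesh to a cube, cone or sphere and applies a red, green, blue or purple material instance to slot 0.
; On BeginPlay it stores the display name of that material as TargetColour, so the colour label comes from the applied material rather than the Colour value.
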(event `self.ReceiveBeginPlay`
  (set `self.TargetColour` (`KismetSystemLibrary.GetDisplayName` (`PrimitiveComponent.GetMaterial` (`self.StaticMesh`) 0))))

(fn `UserConstructionScript`
  (bind _staticmesh (`self.StaticMesh`))
  (bind _staticmesh_2 (`self.StaticMesh`))
  ;[1 1 1] Sets Shape Mesh
  (switch `/Game/Remo/E_Shapes` (`self.Shape`)
    (:`NewEnumerator0`
      (`StaticMeshComponent.SetStaticMesh` _staticmesh_2 "/Game/Remo/Meshes/Cube.Cube"))
    (:`NewEnumerator1`
      (`StaticMeshComponent.SetStaticMesh` _staticmesh_2 "/Game/Remo/Meshes/Cone.Cone"))
    (:`NewEnumerator2`
      (`StaticMeshComponent.SetStaticMesh` _staticmesh_2 "/Game/Remo/Meshes/Sphere.Sphere")))
  ;[1 1 1] Sets Shape Colour
  (switch `/Game/Remo/E_Materials` (`self.Colour`)
    (:`NewEnumerator0`
      (`PrimitiveComponent.SetMaterial` _staticmesh 0 "/Game/Remo/Materials/MI_Red.MI_Red"))
    (:`NewEnumerator1`
      (`PrimitiveComponent.SetMaterial` _staticmesh 0 "/Game/Remo/Materials/MI_Green.MI_Green"))
    (:`NewEnumerator2`
      (`PrimitiveComponent.SetMaterial` _staticmesh 0 "/Game/Remo/Materials/MI_Blue.MI_Blue"))
    (:`NewEnumerator3`
      (`PrimitiveComponent.SetMaterial` _staticmesh 0 "/Game/Remo/Materials/MI_Purple.MI_Purple"))))