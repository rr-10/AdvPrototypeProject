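; Puzzle shape that cycles through coloured materials on a looping timer and counts as an objective on its linked door.
; Construction script sets the mesh and starting colour.
; Melee overlaps and tagged hits share a FlipFlop that pauses or resumes cycling, while CheckColour compares the current material name with TargetShape's target.
; A match turns the spotlight green and completes the door objective once; mismatches alternate timed red feedback with white.
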(event `self.ReceiveBeginPlay`
  (bind _asplayer_fp_character (cast `/Game/MP5/FirstPersonBP/PlayerFP-Character` (`GameplayStatics.GetPlayerCharacter` 0)))
  (set `self.PlayerRef` _asplayer_fp_character)
  (`|ExecutionSequence`
    (:`then_0`
      ;[1 1 1] add one to the objectives number
      (`/Game/MP5/DoorBP.AddObjective` (`self.Which door?`)))
    (:`then_1`
      (bind _returnvalue (`KismetSystemLibrary.K2_SetTimer` null "ChangeColour" (`self.ChangeTime`) true))
      (set `self.Handle` _returnvalue))))

(event `self.Box.OnComponentBeginOverlap`
  (params (OverlappedComponent :type "PrimitiveComponent Object Reference") (OtherActor :type "Actor Object Reference") (OtherComp :type "PrimitiveComponent Object Reference") (OtherBodyIndex :type Integer) (bFromSweep :type Boolean) (SweepResult :type "HitResult Structure (by ref)"))
  ;[0.08683 0.5066 1] Melee interaction
  (if (or (`ActorComponent.ComponentHasTag` OtherComp "Interact") (`ActorComponent.ComponentHasTag` OtherComp "Activator"))
    (if (`/Game/MP5/FirstPersonBP/PlayerFP-Character.Clicked` (`self.PlayerRef`))
      (`KismetSystemLibrary.PrintString` "Melee")
      (`self.CheckColour`)
      ;[1 1 1] Grapple hook attack
      (`/Engine/EditorBlueprintResources/StandardMacros.FlipFlop` :!label _label
        (:`A`
          (`KismetSystemLibrary.K2_ClearAndInvalidateTimerHandle` (`self.Handle`)))
        (:`B`
          (bind _returnvalue (`KismetSystemLibrary.K2_SetTimer` self "ChangeColour" 2.0 true))
          (set `self.Handle` _returnvalue)))
      (else
        (`KismetSystemLibrary.PrintString` "Unlackyyyy")))))

(event `self.ReceiveHit`
  (params (MyComp :type "PrimitiveComponent Object Reference") (Other :type "Actor Object Reference") (OtherComp :type "PrimitiveComponent Object Reference") (bSelfMoved :type Boolean) (HitLocation :type "Vector Structure") (HitNormal :type "Vector Structure") (NormalImpulse :type "Vector Structure") (Hit :type "HitResult Structure (by ref)"))
  ;[1 1 1] Grapple hook attack
  (`self.CheckColour`)
  (if (or (`ActorComponent.ComponentHasTag` OtherComp "Interact") (`ActorComponent.ComponentHasTag` OtherComp "Activator"))
    (goto _label)))

(fn `ChangeColour`
  (bind _staticmesh (`self.StaticMesh`))
  (bind _staticmesh_2 (`self.StaticMesh`))
  (bind _listofmaterials (`self.ListOfMaterials`))
  (bind _staticmesh_3 (`self.StaticMesh`))
  (bind _staticmesh_4 (`self.StaticMesh`))
  (switch `/Game/Remo/Meshes/E_Materials` (`self.Colour`)
    (:`NewEnumerator0`
      (bind _result (`/Engine/EditorBlueprintResources/StandardMacros.IncrementInt` (`self.Index`))
        (:`  `
          (`PrimitiveComponent.SetMaterial` _staticmesh_3 0 (`|GetArrayItem` _listofmaterials _result))
          (set `self.CurrentColour` (`KismetSystemLibrary.GetDisplayName` (`PrimitiveComponent.GetMaterial` _staticmesh_3 0)))
          (set `self.Colour` "NewEnumerator1"))))
    (:`NewEnumerator1`
      (bind _result_2 (`/Engine/EditorBlueprintResources/StandardMacros.IncrementInt` (`self.Index`))
        (:`  `
          (`PrimitiveComponent.SetMaterial` _staticmesh_4 0 (`|GetArrayItem` _listofmaterials _result_2))
          (set `self.CurrentColour` (`KismetSystemLibrary.GetDisplayName` (`PrimitiveComponent.GetMaterial` _staticmesh_4 0)))
          (set `self.Colour` "NewEnumerator2"))))
    (:`NewEnumerator2`
      (bind _result_3 (`/Engine/EditorBlueprintResources/StandardMacros.IncrementInt` (`self.Index`))
        (:`  `
          (`PrimitiveComponent.SetMaterial` _staticmesh 0 (`|GetArrayItem` _listofmaterials _result_3))
          (set `self.CurrentColour` (`KismetSystemLibrary.GetDisplayName` (`PrimitiveComponent.GetMaterial` _staticmesh 0)))
          (set `self.Colour` "NewEnumerator3"))))
    (:`NewEnumerator3`
      (bind _result_4 (`/Engine/EditorBlueprintResources/StandardMacros.IncrementInt` (`self.Index`))
        (:`  `
          (if (> _result_4 (`self.M`))
            (bind _output_get (set `self.Index` 0))
            (`PrimitiveComponent.SetMaterial` _staticmesh_2 0 (`|GetArrayItem` _listofmaterials _output_get))
            (set `self.CurrentColour` (`KismetSystemLibrary.GetDisplayName` (`PrimitiveComponent.GetMaterial` _staticmesh_2 0)))
            (set `self.Colour` "NewEnumerator0")))))))

(fn `CheckColour`
  (locals (ColourHandle :type "TimerHandle Structure"))
  (bind _spotlight (`self.SpotLight`))
  (if (`self.Finished`)
    _
    (elif (`KismetStringLibrary.EqualEqual_StrStr` (`self.CurrentColour`) (`/Game/Remo/BP_TargetShape.TargetColour` (`self.TargetShape`)))
      ;[1 0.3076 0.8269] If the colour matches the target, then the door can open
      (set `self.IsMatching` true)
      (`LightComponent.SetLightColor` _spotlight (struct :`G` 1.0 :`A` 1.0) true)
      (set `self.Finished` true)
      (`/Game/MP5/DoorBP.1objectivedone` (`self.Which door?`))
      (else
        ;[0.3047 0.9002 1] If the colour doesn't match, then...
        (set `self.IsMatching` false)
        (if (`self.HasHit`)
          ;;[0.1679 0.2274 1] If it was paused and hit, shows red and continues with sequence
          (`LightComponent.SetLightColor` _spotlight (struct :`R` 1.0 :`G` 1.0 :`B` 1.0 :`A` 1.0) true)
          (`KismetSystemLibrary.K2_ClearAndInvalidateTimerHandle` (stale _output_get))
          (set `self.HasHit` false)
          (else
            ;;[1 0.3671 0] If it was paused but not hit (var), then shows red and sets to white
            (`LightComponent.SetLightColor` _spotlight (struct :`R` 1.0 :`A` 1.0) true)
            (bind _returnvalue (`KismetSystemLibrary.K2_SetTimer` null "RevertColour" 2.0))
            (bind _output_get (set `local.ColourHandle` _returnvalue))
            (set `self.HasHit` true)))))))

(fn `RevertColour`
  (`LightComponent.SetLightColor` (`self.SpotLight`) (struct :`R` 1.0 :`G` 1.0 :`B` 1.0 :`A` 1.0) true))

(fn `UserConstructionScript`
  (bind _staticmesh (`self.StaticMesh`))
  (bind _staticmesh_2 (`self.StaticMesh`))
  ;[1 1 1] Sets Shape Mesh
  (switch `/Game/Remo/Meshes/E_Shapes` (`self.Shape`)
    (:`NewEnumerator0`
      (`StaticMeshComponent.SetStaticMesh` _staticmesh_2 "/Game/Remo/Meshes/Cube.Cube"))
    (:`NewEnumerator1`
      (`StaticMeshComponent.SetStaticMesh` _staticmesh_2 "/Game/Remo/Meshes/Cone.Cone"))
    (:`NewEnumerator2`
      (`StaticMeshComponent.SetStaticMesh` _staticmesh_2 "/Game/Remo/Meshes/Sphere.Sphere")))
  ;[1 1 1] Sets Shape Colour
  (switch `/Game/Remo/Meshes/E_Materials` (`self.Colour`)
    (:`NewEnumerator0`
      (set `self.Index` 0)
      (`PrimitiveComponent.SetMaterial` _staticmesh 0 "/Game/Remo/Materials/MI_Red.MI_Red"))
    (:`NewEnumerator1`
      (set `self.Index` 1)
      (`PrimitiveComponent.SetMaterial` _staticmesh 0 "/Game/Remo/Materials/MI_Green.MI_Green"))
    (:`NewEnumerator2`
      (set `self.Index` 2)
      (`PrimitiveComponent.SetMaterial` _staticmesh 0 "/Game/Remo/Materials/MI_Blue.MI_Blue"))
    (:`NewEnumerator3`
      (set `self.Index` 3)
      (`PrimitiveComponent.SetMaterial` _staticmesh 0 "/Game/Remo/Materials/MI_Purple.MI_Purple"))))