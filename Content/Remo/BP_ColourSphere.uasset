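; Colour puzzle sphere that cycles through red, green, blue and purple materials and flags whether it matches its TargetSphere's colour.
; A looping timer runs ChangeColour, and hits from Interact-tagged components alternately stop and restart it, restarting at a fixed interval rather than ChangeTime.
; Tick compares the current material's display name with the target to set IsMatching.
; The construction script previews the starting colour in the editor.
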(event `self.ReceiveBeginPlay`
  (bind _returnvalue (`KismetSystemLibrary.K2_SetTimer` null "ChangeColour" (`self.ChangeTime`) true))
  (set `self.Handle` _returnvalue))

(event `self.ReceiveTick`
  (params (DeltaSeconds :type "Float (single-precision)"))
  (`self.CheckColour`))

(event `self.ReceiveHit`
  (params (MyComp :type "PrimitiveComponent Object Reference") (Other :type "Actor Object Reference") (OtherComp :type "PrimitiveComponent Object Reference") (bSelfMoved :type Boolean) (HitLocation :type "Vector Structure") (HitNormal :type "Vector Structure") (NormalImpulse :type "Vector Structure") (Hit :type "HitResult Structure (by ref)"))
  (bind _returnvalue (`ActorComponent.ComponentHasTag` OtherComp "Interact"))
  (`KismetSystemLibrary.PrintString` (`KismetStringLibrary.Conv_BoolToString` _returnvalue))
  (if _returnvalue
    (`/Engine/EditorBlueprintResources/StandardMacros.FlipFlop`
      (:`A`
        (`KismetSystemLibrary.K2_ClearAndInvalidateTimerHandle` (`self.Handle`)))
      (:`B`
        (bind _returnvalue_2 (`KismetSystemLibrary.K2_SetTimer` self "ChangeColour" 2.0 true))
        (set `self.Handle` _returnvalue_2)))))

(fn `ChangeColour`
  (bind _listofmaterials (`self.ListOfMaterials`))
  (bind _shape (`self.Shape`))
  (bind _shape_2 (`self.Shape`))
  (bind _shape_3 (`self.Shape`))
  (bind _shape_4 (`self.Shape`))
  (switch `/Game/Remo/Meshes/E_Materials` (`self.Colour`)
    (:`NewEnumerator0`
      (bind _result (`/Engine/EditorBlueprintResources/StandardMacros.IncrementInt` (`self.Index`))
        (:`  `
          (`PrimitiveComponent.SetMaterial` _shape_2 0 (`|GetArrayItem` _listofmaterials _result))
          (set `self.CurrentColour` (`KismetSystemLibrary.GetDisplayName` (`PrimitiveComponent.GetMaterial` _shape_2 0)))
          (set `self.Colour` "NewEnumerator1"))))
    (:`NewEnumerator1`
      (bind _result_2 (`/Engine/EditorBlueprintResources/StandardMacros.IncrementInt` (`self.Index`))
        (:`  `
          (`PrimitiveComponent.SetMaterial` _shape_3 0 (`|GetArrayItem` _listofmaterials _result_2))
          (set `self.CurrentColour` (`KismetSystemLibrary.GetDisplayName` (`PrimitiveComponent.GetMaterial` _shape_3 0)))
          (set `self.Colour` "NewEnumerator2"))))
    (:`NewEnumerator2`
      (bind _result_3 (`/Engine/EditorBlueprintResources/StandardMacros.IncrementInt` (`self.Index`))
        (:`  `
          (`PrimitiveComponent.SetMaterial` _shape_4 0 (`|GetArrayItem` _listofmaterials _result_3))
          (set `self.CurrentColour` (`KismetSystemLibrary.GetDisplayName` (`PrimitiveComponent.GetMaterial` _shape_4 0)))
          (set `self.Colour` "NewEnumerator3"))))
    (:`NewEnumerator3`
      (bind _result_4 (`/Engine/EditorBlueprintResources/StandardMacros.IncrementInt` (`self.Index`))
        (:`  `
          (if (> _result_4 (`self.M`))
            (bind _output_get (set `self.Index` 0))
            (`PrimitiveComponent.SetMaterial` _shape 0 (`|GetArrayItem` _listofmaterials _output_get))
            (set `self.CurrentColour` (`KismetSystemLibrary.GetDisplayName` (`PrimitiveComponent.GetMaterial` _shape 0)))
            (set `self.Colour` "NewEnumerator0")))))))

(fn `CheckColour`
  (if (`KismetStringLibrary.EqualEqual_StrStr` (`self.CurrentColour`) (`/Game/Remo/BP_TargetSphere.TargetColour` (`self.TargetSphere`)))
    (set `self.IsMatching` true)
    (else
      (set `self.IsMatching` false))))

(fn `UserConstructionScript`
  (bind _shape (`self.Shape`))
  ;[0.3369 0.5168 1] Sets Colours in Editor Mode
  (switch `/Game/Remo/Meshes/E_Materials` (`self.Colour`)
    (:`NewEnumerator0`
      (set `self.Index` 0)
      (`PrimitiveComponent.SetMaterial` _shape 0 "/Game/Remo/Materials/MI_Red.MI_Red"))
    (:`NewEnumerator1`
      (set `self.Index` 1)
      (`PrimitiveComponent.SetMaterial` _shape 0 "/Game/Remo/Materials/MI_Green.MI_Green"))
    (:`NewEnumerator2`
      (set `self.Index` 2)
      (`PrimitiveComponent.SetMaterial` _shape 0 "/Game/Remo/Materials/MI_Blue.MI_Blue"))
    (:`NewEnumerator3`
      (set `self.Index` 3)
      (`PrimitiveComponent.SetMaterial` _shape 0 "/Game/Remo/Materials/MI_Purple.MI_Purple"))))