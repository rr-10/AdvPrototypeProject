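; BP_CompletedShape is a puzzle completion indicator that reacts when its target shapes are matched.
; Every Tick it loops over TargetShapes, copying each Matched state into AllMatching, so the last element alone determines the final value.
; When that flag is true, it turns its Sphere orange and uses a DoOnce to play the puzzle-complete sound a single time.
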(event `self.ReceiveBeginPlay`)

(event `self.ReceiveTick`
  (params (DeltaSeconds :type "Float (single-precision)"))
  (for _array_element (`self.TargetShapes`)
    (if (`/Game/Remo/BP_TargetShape.Matched` _array_element)
      (set `self.AllMatching` true)
      (else
        (set `self.AllMatching` false))))
  (if (`self.AllMatching`)
    (`PrimitiveComponent.SetMaterial` (`self.Sphere`) 0 "/Game/Remo/Materials/MI_Orange.MI_Orange")
    (`/Engine/EditorBlueprintResources/StandardMacros.DoOnce` false
      (:`Completed`
        (`GameplayStatics.PlaySound2D` "/Game/SarahRoddam_AudioAndSubtitles/SFX_Puzzles/SFX_PuzzleComplete_Cue.SFX_PuzzleComplete_Cue" 1.0 1.0 0.0 null null)))))

(fn `UserConstructionScript`)