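; BP_TargetSphere is a target sphere actor that comes in red, green, blue or purple.
; The Construction Script maps the Colour selection to a matching material instance on slot 0 of its static mesh.
; On BeginPlay it stores that material's display name in TargetColour, so the recorded colour derives from the applied material rather than the Colour value.
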(event `self.ReceiveBeginPlay`
  (set `self.TargetColour` (`KismetSystemLibrary.GetDisplayName` (`PrimitiveComponent.GetMaterial` (`self.StaticMeshComponent`) 0))))

(fn `UserConstructionScript`
  (bind _staticmeshcomponent (`self.StaticMeshComponent`))
  (switch `/Game/Remo/Meshes/E_Materials` (`self.Colour`)
    (:`NewEnumerator0`
      (`PrimitiveComponent.SetMaterial` _staticmeshcomponent 0 "/Game/Remo/Materials/MI_Red.MI_Red"))
    (:`NewEnumerator1`
      (`PrimitiveComponent.SetMaterial` _staticmeshcomponent 0 "/Game/Remo/Materials/MI_Green.MI_Green"))
    (:`NewEnumerator2`
      (`PrimitiveComponent.SetMaterial` _staticmeshcomponent 0 "/Game/Remo/Materials/MI_Blue.MI_Blue"))
    (:`NewEnumerator3`
      (`PrimitiveComponent.SetMaterial` _staticmeshcomponent 0 "/Game/Remo/Materials/MI_Purple.MI_Purple"))))