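; BP_Mace_Trap is a trap actor that swings continuously from BeginPlay and damages what it hits.
; A timeline drives a rotator lerp on the Scene component's relative rotation between two opposite angles, replaying from the start whenever it finishes.
; Overlaps with the Box component apply fixed damage to the other actor, except when the overlapping component carries the "Activator" tag.
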(event `self.ReceiveBeginPlay`
  (`self.Swing`))

(event `Swing`
  (bind (_direction _newtrack_1) (`Timeline|Time` :!via `PlayFromStart`)
    (:`Update`
      (`SceneComponent.K2_SetRelativeRotation` (`self.Scene`) (`KismetMathLibrary.RLerp` (struct :`Pitch` -40.0) (struct :`Pitch` 40.0) _newtrack_1 true) false false))
    (:`Finished`
      (`self.Swing`))))

(event `self.Box.OnComponentBeginOverlap`
  (params (OverlappedComponent :type "PrimitiveComponent Object Reference") (OtherActor :type "Actor Object Reference") (OtherComp :type "PrimitiveComponent Object Reference") (OtherBodyIndex :type Integer) (bFromSweep :type Boolean) (SweepResult :type "HitResult Structure (by ref)"))
  (if (not (`ActorComponent.ComponentHasTag` OtherComp "Activator"))
    (`GameplayStatics.ApplyDamage` OtherActor 100.0)))

(fn `UserConstructionScript`)