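; BP_Spike_Trap is a looping spike hazard that damages actors touching its box.
; From BeginPlay, a timeline slides the mesh along its local X axis, then restarts after a short delay.
; Box overlaps deal 100 damage and play a 2D spike death sound, unless the overlapping component is tagged Activator.
; The sound plays on each such overlap, with no check that the actor died.
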(event `self.ReceiveBeginPlay`
  (`self.Spike`))

(event `Spike`
  (bind (_direction _newtrack_1) (`Timeline|Time` :!via `PlayFromStart`)
    (:`Update`
      (`SceneComponent.K2_SetRelativeLocation` (`self.StaticMesh`) (`KismetMathLibrary.VLerp` (0.0 0.0 0.0) (70.0 0.0 0.0) _newtrack_1) false false))
    (:`Finished`
      (`KismetSystemLibrary.Delay` 0.9)
      (`self.Spike`))))

(event `self.Box.OnComponentBeginOverlap`
  (params (OverlappedComponent :type "PrimitiveComponent Object Reference") (OtherActor :type "Actor Object Reference") (OtherComp :type "PrimitiveComponent Object Reference") (OtherBodyIndex :type Integer) (bFromSweep :type Boolean) (SweepResult :type "HitResult Structure (by ref)"))
  (if (not (`ActorComponent.ComponentHasTag` OtherComp "Activator"))
    (`GameplayStatics.ApplyDamage` OtherActor 100.0)
    ;[1 1 1] play spike death sound (Sarah)
    (`GameplayStatics.PlaySound2D` "/Game/SarahRoddam_AudioAndSubtitles/SFX_Player/SFX_SpikeDeath_Cue.SFX_SpikeDeath_Cue" 1.0 1.0 0.0 null null)))

(fn `UserConstructionScript`)