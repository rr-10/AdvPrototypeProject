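; CheckPoint1 is a one-shot checkpoint actor that records a respawn point when the player overlaps its box.
; It stores its own location raised along Z, plus the player's rotation and scale, on PlayerFP-Character and sets that character's checkpoint flag.
; Activation shows a prompt widget and plays a sound while a timeline offsets the actor's height and yaw.
; When the timeline finishes, the prompt is removed and the actor destroys itself.
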(event `self.Box.OnComponentBeginOverlap`
  (params (OverlappedComponent :type "PrimitiveComponent Object Reference") (OtherActor :type "Actor Object Reference") (OtherComp :type "PrimitiveComponent Object Reference") (OtherBodyIndex :type Integer) (bFromSweep :type Boolean) (SweepResult :type "HitResult Structure (by ref)"))
  (bind (_returnvalue_roll _returnvalue_pitch _returnvalue_yaw) (`KismetMathLibrary.BreakRotator` (`self.K2_GetActorRotation`)))
  (bind (_returnvalue_x _returnvalue_y _returnvalue_z) (`KismetMathLibrary.BreakVector` (`self.K2_GetActorLocation`)))
  (bind _returnvalue (`self.GetTransform`))
  (bind _asplayer_fp_character (cast `/Game/MP5/FirstPersonBP/PlayerFP-Character` OtherActor))
  (if (not (`self.Once`))
    ;[1 1 1] add and remove prompt from screen
    (set `self.Once` true)
    (bind _returnvalue_2 (`|CreateWidget` "/Game/MP5/Prompt/CheckpointPrompt-Widget.CheckpointPrompt-Widget_C"))
    (`UserWidget.AddToViewport` _returnvalue_2 0)
    (bind (_returnvalue_location _returnvalue_rotation _returnvalue_scale) (`KismetMathLibrary.BreakTransform` (`self.GetTransform` _asplayer_fp_character)))
    (set `/Game/MP5/FirstPersonBP/PlayerFP-Character.Checkpoint_transform` (`KismetMathLibrary.MakeTransform` (`KismetMathLibrary.MakeVector` _returnvalue_x _returnvalue_y (+ _returnvalue_z 200.0)) _returnvalue_rotation _returnvalue_scale) _asplayer_fp_character)
    (set `/Game/MP5/FirstPersonBP/PlayerFP-Character.Checkpoint` true _asplayer_fp_character)
    (set `/Game/MP5/FirstPersonBP/PlayerFP-Character.CheckPoint_rotation` (`self.K2_GetActorRotation` _asplayer_fp_character) _asplayer_fp_character)
    (`KismetSystemLibrary.PrintString` "CheckPoint")
    (set `self.ActorZ` (.z (.location _returnvalue)))
    (set `self.RotateY` _returnvalue_yaw)
    (`GameplayStatics.PlaySoundAtLocation` "/Game/Liam/CheckPoint.CheckPoint" (`KismetMathLibrary.MakeVector` (.x (.location _returnvalue)) (.y (.location _returnvalue)) (.z (.location _returnvalue))) (struct) 1.0 1.0 0.0 null null null)
    (bind (_direction _track) (`Timeline|Timeline_0` :!via `PlayFromStart`)
      (:`Update`
        (`self.K2_SetActorLocation` (`KismetMathLibrary.MakeVector` (.x (.location _returnvalue)) (.y (.location _returnvalue)) (- (`self.ActorZ`) _track)))
        (`self.K2_SetActorRotation` (`KismetMathLibrary.MakeRotator` _returnvalue_roll _returnvalue_pitch (- (`self.RotateY`) _track))))
      (:`Finished`
        (`Widget.RemoveFromParent` _returnvalue_2)
        (`self.K2_DestroyActor`)))))

(fn `UserConstructionScript`)