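; Red Light, Green Light minigame that kills the first-person player for moving on red until they reach the End trigger.
; A looping timer drives timeline TL_LightCycle, whose event tracks flash a warning and switch the wall panel's material and sound.
; During red, a timer polls raw movement and jump keys rather than velocity, setting Detected for the timeline update to punish.
; Overlapping End stops the cycle and turns the panel blue.
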(event `self.ReceiveBeginPlay`
  (bind _returnvalue (`KismetSystemLibrary.K2_SetTimerDelegate` (delegate `LightCycle`) 0.01 true))
  (set `self.MainCycleTimer` _returnvalue))

(event `LightCycle`
  (`Timeline|TL_LightCycle` :!label _label
    (:`Update`
      (if (`self.Detected`)
        (`self.PunishMovement`)))
    (:`Finished`
      (`self.ResetTimeline`))
    (:`StartFlashing`
      (bind _returnvalue (`KismetSystemLibrary.K2_SetTimer` null "FlashColour" 0.2 true))
      (set `self.FlashingTimer` _returnvalue))
    (:`ChangeToRed`
      (`self.ChangeToRed`)
      (bind _returnvalue_2 (`KismetSystemLibrary.K2_SetTimer` null "CheckForMovement" 0.1 true))
      (set `self.MovementTimer` _returnvalue_2))
    (:`ChangeToGreen`
      (`KismetSystemLibrary.K2_ClearAndInvalidateTimerHandle` (`self.MovementTimer`))
      (`self.ChangeToGreen`))))

(event `CancelTimeline`
  (goto _label :!via `Stop`))

(event `ResetTimeline`
  (goto _label :!via `SetNewTime`))

(event `self.End.OnComponentBeginOverlap`
  (params (OverlappedComponent :type "PrimitiveComponent Object Reference") (OtherActor :type "Actor Object Reference") (OtherComp :type "PrimitiveComponent Object Reference") (OtherBodyIndex :type Integer) (bFromSweep :type Boolean) (SweepResult :type "HitResult Structure (by ref)"))
  (set `self.EndReached` true)
  (`KismetSystemLibrary.K2_ClearAndInvalidateTimerHandle` (`self.MainCycleTimer`))
  (`KismetSystemLibrary.K2_ClearAndInvalidateTimerHandle` (`self.MovementTimer`))
  (`self.CancelTimeline`)
  (`PrimitiveComponent.SetMaterial` (`self.WallPanel`) 0 "/Game/Remo/Materials/MI_Blue.MI_Blue"))

(fn `ChangeToGreen`
  (`PrimitiveComponent.SetMaterial` (`self.WallPanel`) 0 "/Game/Remo/Materials/MI_Green.MI_Green")
  (`GameplayStatics.PlaySound2D` "/Game/SarahRoddam_AudioAndSubtitles/SFX_Puzzles/SFX_RedGreenLight_Go.SFX_RedGreenLight_Go" 1.0 1.0 0.0 null null))

(fn `ChangeToRed`
  (`PrimitiveComponent.SetMaterial` (`self.WallPanel`) 0 "/Game/Remo/Materials/MI_Red.MI_Red")
  (`GameplayStatics.PlaySound2D` "/Game/SarahRoddam_AudioAndSubtitles/SFX_Puzzles/SFX_RedGreenLight_Stop.SFX_RedGreenLight_Stop" 1.0 1.0 0.0 null null))

(fn `CheckForMovement`
  (bind _returnvalue (`GameplayStatics.GetPlayerController` 0))
  (if (and (not (`self.EndReached`)) (or (`PlayerController.IsInputKeyDown` _returnvalue "W") (`PlayerController.IsInputKeyDown` _returnvalue "S") (`PlayerController.IsInputKeyDown` _returnvalue "A") (`PlayerController.IsInputKeyDown` _returnvalue "D") (`PlayerController.IsInputKeyDown` _returnvalue "SpaceBar")))
    (set `self.Detected` true)))

(fn `FlashColour`
  (bind _wallpanel (`self.WallPanel`))
  (bind _returnvalue (`PrimitiveComponent.GetMaterial` (`self.WallPanel`) 0))
  (if (not (`self.EndReached`))
    (`GameplayStatics.PlaySound2D` "/Game/SarahRoddam_AudioAndSubtitles/SFX_Puzzles/SFX_RedGreenLight_Countdown_Cue.SFX_RedGreenLight_Countdown_Cue" 1.0 1.0 0.0 null null)
    (if (or (== _returnvalue "/Game/Remo/Materials/MI_Green.MI_Green") (== _returnvalue "/Game/Remo/Materials/MI_Red.MI_Red"))
      (`PrimitiveComponent.SetMaterial` _wallpanel 0 "/Game/Remo/Materials/MI_yellow.MI_Yellow")
      (else
        (`PrimitiveComponent.SetMaterial` _wallpanel 0 "/Game/Remo/Materials/MI_Red.MI_Red")))
    (bind _result (`/Engine/EditorBlueprintResources/StandardMacros.IncrementInt` (`self.TimesFlashed`))
      (:`  `
        ;[1 1 1] Reset when done with flashing pattern
        (if (>= _result 5)
          (set `self.TimesFlashed` 0)
          (`KismetSystemLibrary.K2_ClearAndInvalidateTimerHandle` (`self.FlashingTimer`)))))))

(fn `UserConstructionScript`)