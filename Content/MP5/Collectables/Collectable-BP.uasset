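; Collectable pickup actor that optionally spins on Tick and reacts when the first-person player overlaps it.
; Overlap records a Collectables stat, calls CollectedKey on the player and enables input.
; With AutoCollect, it shows a widget, destroys itself, awards and records EXP, saves the game and plays a sound.
; Interact prompt, manual-collect countdown and timeline rotation logic are disconnected, so non-auto pickups never finish collecting.
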(event `self.ReceiveTick`
  (params (DeltaSeconds :type "Float (single-precision)"))
  (if (`self.Rotating`)
    (`SceneComponent.K2_SetRelativeRotation` (`self.DefaultSceneRoot`) (`KismetMathLibrary.MakeRotator` (.roll (`SceneComponent.K2_GetComponentRotation` (`self.DefaultSceneRoot`))) (.pitch (`SceneComponent.K2_GetComponentRotation` (`self.DefaultSceneRoot`))) (+ (.yaw (`SceneComponent.K2_GetComponentRotation` (`self.DefaultSceneRoot`))) (`self.Speed`))) false false)))

(event `self.ReceiveBeginPlay`)

(event `self.Overlapping.OnComponentBeginOverlap`
  (params (OverlappedComponent :type "PrimitiveComponent Object Reference") (OtherActor :type "Actor Object Reference") (OtherComp :type "PrimitiveComponent Object Reference") (OtherBodyIndex :type Integer) (bFromSweep :type Boolean) (SweepResult :type "HitResult Structure (by ref)"))
  (bind _addedexp (`self.AddedEXP`))
  (bind _asplayer_fp_character (cast `/Game/MP5/FirstPersonBP/PlayerFP-Character` OtherActor))
  (`/Game/DanaSawdon/Blueprints/StatsTrackerLibrary.AddStat` "Collectables" 50.0)
  (`/Game/MP5/FirstPersonBP/PlayerFP-Character.CollectedKey` _asplayer_fp_character)
  (`self.EnableInput` (`GameplayStatics.GetPlayerController` 0))
  (if (`self.Auto Collect`)
    (bind _returnvalue (`|CreateWidget` "/Game/MP5/Collectables/CollectableWidget.CollectableWidget_C"))
    (`UserWidget.AddToViewport` _returnvalue 0)
    (`self.K2_DestroyActor`)
    (set `self.HasPicked` true)
    ;[1 1 1] Add EXP
    (bind _asplayer_fp_character_2 (cast `/Game/MP5/FirstPersonBP/PlayerFP-Character` (`GameplayStatics.GetPlayerCharacter` 0)))
    (`/Game/MP5/FirstPersonBP/PlayerFP-Character.AddEXP` _asplayer_fp_character_2 _addedexp)
    (`/Game/DanaSawdon/Blueprints/StatsTrackerLibrary.AddStat` "EXP" (`KismetMathLibrary.Conv_IntToDouble` _addedexp))
    (`/Game/MP5/FirstPersonBP/PlayerFP-Character.SaveGame` _asplayer_fp_character_2 (`self.Slot Name`) true)
    ;[1 1 1] play collectible sound. (Sarah)
    (`GameplayStatics.PlaySound2D` (`self.Collection sound`) 1.0 1.0 0.0 null null)))

(event `self.Overlapping.OnComponentEndOverlap`
  (params (OverlappedComponent :type "PrimitiveComponent Object Reference") (OtherActor :type "Actor Object Reference") (OtherComp :type "PrimitiveComponent Object Reference") (OtherBodyIndex :type Integer))
  (cast `/Game/MP5/FirstPersonBP/PlayerFP-Character` OtherActor)
  (`self.DisableInput` (`GameplayStatics.GetPlayerController` 0)))

(fn `UserConstructionScript`)