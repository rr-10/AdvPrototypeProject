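; Level door actor that opens on objective count, unlocked maps or player level, and can act as a level exit.
; Objective events, BeginPlay and the activation overlap run the checks, feeding timeline macros that swing or slide the mesh and hide locked signage.
; When enabled, the NextLVL trigger records unlocked and completed maps on the player, shows a loading widget, then opens the destination, incrementing LevelCount for hub destinations.
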(event `InputAction|Interact`
  (params (Key :type "Key Structure"))
  ;[1 1 1] Open door if close and collectables collected
)

(event `self.DoorActivation.OnComponentEndOverlap`
  (params (OverlappedComponent :type "PrimitiveComponent Object Reference") (OtherActor :type "Actor Object Reference") (OtherComp :type "PrimitiveComponent Object Reference") (OtherBodyIndex :type Integer))
  ;[1 1 1] Open door if close and collectables collected
)

(event `hub opens`
  ;[1 1 1] when hub level opens, add one to the door level (Rob)
  (bind _asplayer_fp_character (cast `/Game/MP5/FirstPersonBP/PlayerFP-Character` (`GameplayStatics.GetPlayerCharacter` 0)))
  (set `/Game/MP5/FirstPersonBP/PlayerFP-Character.Level count` (+ (`/Game/MP5/FirstPersonBP/PlayerFP-Character.Level count` _asplayer_fp_character) 1) _asplayer_fp_character))

(event `self.ReceiveBeginPlay`
  (bind _staticmesh (`self.StaticMesh`))
  (bind _chains (`self.Chains`))
  (bind _chains_2 (`self.Chains`))
  (bind (_returnvalue_x _returnvalue_y) (`KismetMathLibrary.BreakVector` (`SceneComponent.K2_GetComponentLocation` (`self.SlidingPointer`))))
  (bind _returnvalue (`SceneComponent.K2_GetComponentLocation` _staticmesh))
  ;[1 1 1] Objectives counters
  ;;[1 1 1] Check at start if u can open door
  (bind _asplayer_fp_character (cast `/Game/MP5/FirstPersonBP/PlayerFP-Character` (`GameplayStatics.GetPlayerCharacter` 0)))
  (set `self.TargetPlayer` _asplayer_fp_character)
  (`|ExecutionSequence`
    (:`then_0`
      (if (not (`self.Locked`)) :!label _label
        ;;[1 1 1] Open the door if done
        (bind _output_get (set `self.Open-Closed` (>= (`self.ObjectiveCounter`) (`self.Number of Objectives`))))
        ;[1 1 1] Openning doors if unlocked
        (if (and _output_get (`self.Automatic`))
          (if (`KismetSystemLibrary.IsValid` _chains)
            (`SceneComponent.SetHiddenInGame` _chains true false))
          (`SceneComponent.SetHiddenInGame` (`self.ClosedSign`) true false)
          (`SceneComponent.SetHiddenInGame` (`self.locked_text`) true false)
          (if (`self.AlreadyOpened`)
            _
            (elif (`self.SlidingDoor`)
              (bind (_direction _doortrack) (`Timeline|Timeline_2`)
                (:`Update`
                  (`SceneComponent.K2_SetWorldLocation` _staticmesh (`KismetMathLibrary.VLerp` _returnvalue (`KismetMathLibrary.MakeVector` (.x _returnvalue) _returnvalue_y (.z _returnvalue)) _doortrack) false false))
                (:`Finished`
                  (set `self.AlreadyOpened` true :!label _label_2)))
              (else
                (bind (_direction_2 _doortrack_2) (`Timeline|Timeline_0`)
                  (:`Update`
                    (`SceneComponent.K2_SetRelativeRotation` (`self.StaticMesh`) (`KismetMathLibrary.MakeRotator` 0.0 0.0 (`KismetMathLibrary.Lerp` (`self.Closed Angle`) (`self.Open Angle`) _doortrack_2)) false false))
                  (:`Finished`
                    (goto _label_2)))))))))
    (:`then_1`
      (bind _unlockedmaps (`/Game/MP5/FirstPersonBP/PlayerFP-Character.GetUnlockedMaps` (`self.TargetPlayer`) :!label _label_3))
      (if (`KismetArrayLibrary.Array_Contains` _unlockedmaps (`self.Destination Level Name`))
        (set `self.Locked` false)
        (set `self.Open-Closed` true)))
    (:`then_2`
      (if (or (`self.Open-Closed`) (>= (`/Game/MP5/FirstPersonBP/PlayerFP-Character.Level` (`self.TargetPlayer`)) (`self.LEVELtoOpen`))) :!label _label_4
        (if (`KismetSystemLibrary.IsValid` _chains_2)
          (`SceneComponent.SetHiddenInGame` _chains_2 true false))
        (`SceneComponent.SetHiddenInGame` (`self.ClosedSign`) true false)
        (`SceneComponent.SetHiddenInGame` (`self.locked_text`) true false)
        (if (`self.AlreadyOpened`)
          ;[1 1 1] Sara SFX
          (`/Engine/EditorBlueprintResources/StandardMacros.DoOnce` false :!label _label_5
            (:`Completed`
              (`GameplayStatics.PlaySound2D` null 1.0 1.0 0.0 null null)
              (`KismetSystemLibrary.Delay` 3.0)
              (goto _label_5 :!via `Reset`)))
          (elif (`self.SlidingDoor`)
            (bind (_direction_3 _doortrack_3) (`Timeline|Timeline_4`)
              (:`Update`
                (`SceneComponent.K2_SetRelativeLocation` (`self.StaticMesh`) (0.0 0.0 0.0) false false))
              (:`Finished`
                (set `self.AlreadyOpened` true :!label _label_6)
                (goto _label_5)))
            (else
              (bind (_direction_4 _doortrack_4) (`Timeline|Timeline_3`)
                (:`Update`
                  (`SceneComponent.K2_SetRelativeRotation` (`self.StaticMesh`) (`KismetMathLibrary.MakeRotator` 0.0 0.0 (`KismetMathLibrary.Lerp` (`self.Closed Angle`) (`self.Open Angle`) _doortrack_4)) false false))
                (:`Finished`
                  (goto _label_6))))))))
    (:`then_3`
      ;[1 1 1] Indicator Arrow
      (if (`self.Indicator`)
        (`SceneComponent.SetHiddenInGame` (`self.IndicatorArrowMesh`) false false)))
    (:`then_4`
      ;[1 1 1] Door Indicator
      (if (`self.LeadstoNextLVL`)
        (if (!= (`KismetArrayLibrary.Array_Find` (`/Game/MP5/FirstPersonBP/PlayerFP-Character.UnlockedMaps` (`self.TargetPlayer`)) (`self.Destination Level Name`)) -1)
          (`SceneComponent.SetHiddenInGame` (`self.IndicatorArrowMesh`) true false))))
    (:`then_5`
      ;[1 1 1] Sidewalls visible
      (if (`self.DoorsSidewallsVisibility`)
        (`SceneComponent.SetHiddenInGame` (`self.leftwall`) false false)
        (`SceneComponent.SetHiddenInGame` (`self.rightwall`) false false)))
    (:`then_6`
      ;[1 1 1] Delete sidewalls
      (if (`self.Nosidewalls`)
        (`ActorComponent.K2_DestroyComponent` (`self.leftwall`))
        (`ActorComponent.K2_DestroyComponent` (`self.rightwall`))))
    (:`then_7`
      ;[1 1 1] Deactivate fog
      (if (`self.NoFog`)
        (`ActorComponent.Deactivate` (`self.LocalFog_PS_2`))))
    (:`then_8`
      ;[1 1 1] Destroy chains
      (if (`self.Open-Closed`)
        (`ActorComponent.K2_DestroyComponent` (`self.Chains`))))))

(event `1objectivedone`
  ;[1 1 1] Objectives counters
  ;;[1 1 1] Add to completed objects
  (`/Engine/EditorBlueprintResources/StandardMacros.IncrementInt` (`self.ObjectiveCounter`)
    (:`  `
      (goto _label))))

(event `Pris opens`
  ;[1 1 1] when hub level opens, add one to the door level (Rob)
  (bind _asplayer_fp_character (cast `/Game/MP5/FirstPersonBP/PlayerFP-Character` (`GameplayStatics.GetPlayerCharacter` 0)))
  (set `/Game/MP5/FirstPersonBP/PlayerFP-Character.Level count` (+ (`/Game/MP5/FirstPersonBP/PlayerFP-Character.Level count` _asplayer_fp_character) 1) _asplayer_fp_character))

(event `AddObjective`
  ;[1 1 1] Objectives counters
  ;;[1 1 1] Add to number of objectives to be completed
  (`/Engine/EditorBlueprintResources/StandardMacros.IncrementInt` (`self.Number of Objectives`)
    (:`  `
      (goto _label))))

(event `self.DoorActivation.OnComponentBeginOverlap`
  (params (OverlappedComponent :type "PrimitiveComponent Object Reference") (OtherActor :type "Actor Object Reference") (OtherComp :type "PrimitiveComponent Object Reference") (OtherBodyIndex :type Integer) (bFromSweep :type Boolean) (SweepResult :type "HitResult Structure (by ref)"))
  (`|ExecutionSequence`
    (:`then_0`
      (goto _label_3))
    (:`then_1`
      (if (== OtherActor (`self.TargetPlayer`))
        (goto _label_4)))))

(event `self.NextLVL.OnComponentBeginOverlap`
  (params (OverlappedComponent :type "PrimitiveComponent Object Reference") (OtherActor :type "Actor Object Reference") (OtherComp :type "PrimitiveComponent Object Reference") (OtherBodyIndex :type Integer) (bFromSweep :type Boolean) (SweepResult :type "HitResult Structure (by ref)"))
  (bind _destination_level_name (`self.Destination Level Name`))
  ;[1 1 1] Check if its the player
  (if (and (and (== (`self.TargetPlayer`) OtherActor) (`ActorComponent.ComponentHasTag` OtherComp "Playermesh")) (`self.LeadstoNextLVL`))
    ;[1 1 1] Save the unlocked map
    (`/Game/MP5/FirstPersonBP/PlayerFP-Character.AddtoUnlockedMaps` (`self.TargetPlayer`) (`self.MapsToUnlock`))
    ;[1 1 1] Add Completed Level
    (bind _returnvalue (`GameplayStatics.GetCurrentLevelName` true))
    (`/Game/MP5/FirstPersonBP/PlayerFP-Character.Add too completed levesls` (`self.TargetPlayer`) (`KismetStringLibrary.Conv_StringToName` _returnvalue))
    ;[0.512 1 0.5012] Load the next lvl Dana
    (bind _returnvalue_2 (`|CreateWidget` "/Game/DanaSawdon/MainMenu/Loading_Widget.Loading_Widget_C" (`GameplayStatics.GetPlayerController` 0)))
    (`UserWidget.AddToViewport` _returnvalue_2 0)
    (`KismetSystemLibrary.Delay` 2.0)
    (`Widget.RemoveFromParent` _returnvalue_2)
    (switch `name` _destination_level_name
      (:`Default`
        (`GameplayStatics.OpenLevel` _destination_level_name))
      (:`HUB_world`
        (`self.hub opens`)
        (`GameplayStatics.OpenLevel` "HUB_world"))
      (:`HUB_Prison`
        (`self.Pris opens`)
        (`GameplayStatics.OpenLevel` "HUB_Prison")))))

(fn `IsOpen`
  (returns (Isopen :type Boolean))
  (return (`self.Open-Closed`)))

(fn `UserConstructionScript`)