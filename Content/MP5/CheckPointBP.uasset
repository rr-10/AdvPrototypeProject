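; Checkpoint actor that saves the player's respawn point when the player walks into its trigger box.
; On overlap, it casts to PlayerFP-Character, stores that character's current transform and rotation on it and sets its checkpoint flag.
; It then prints a debug message and shows a CheckpointPromptWidget on screen, removing it after a short delay.
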(event `self.Box.OnComponentBeginOverlap`
  (params (OverlappedComponent :type "PrimitiveComponent Object Reference") (OtherActor :type "Actor Object Reference") (OtherComp :type "PrimitiveComponent Object Reference") (OtherBodyIndex :type Integer) (bFromSweep :type Boolean) (SweepResult :type "HitResult Structure (by ref)"))
  (bind _asplayer_fp_character (cast `/Game/MP5/FirstPersonBP/PlayerFP-Character` OtherActor))
  (set `/Game/MP5/FirstPersonBP/PlayerFP-Character.Checkpoint_transform` (`self.GetTransform` _asplayer_fp_character) _asplayer_fp_character)
  (set `/Game/MP5/FirstPersonBP/PlayerFP-Character.Checkpoint` true _asplayer_fp_character)
  (set `/Game/MP5/FirstPersonBP/PlayerFP-Character.CheckPoint_rotation` (`self.K2_GetActorRotation` _asplayer_fp_character) _asplayer_fp_character)
  (`KismetSystemLibrary.PrintString` "CheckPoint")
  ;[1 1 1] add and remove prompt from screen
  (bind _returnvalue (`|CreateWidget` "/Game/MP5/Prompt/CheckpointPrompt-Widget.CheckpointPrompt-Widget_C"))
  (`UserWidget.AddToViewport` _returnvalue 0)
  (`KismetSystemLibrary.Delay` 2.0)
  (`Widget.RemoveFromParent` _returnvalue))

(fn `UserConstructionScript`)